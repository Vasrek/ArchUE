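; BP_House is a checkpoint actor that can also act as the level's end goal when flagged as the last checkpoint.
; When a BP_Knight overlaps its Box, a regular checkpoint copies the SMPotato component's world transform into the knight's SpawnTransform.
; The last checkpoint instead shows the WB_Win widget, waits briefly, then opens the level named by LevelName.
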(event OnComponentBeginOverlap(Box)
  (params (OverlappedComponent :type Primitive%20Component%20Object%20Reference) (OtherActor :type Actor%20Object%20Reference) (OtherComp :type Primitive%20Component%20Object%20Reference) (OtherBodyIndex :type Integer) (bFromSweep :type Boolean) (SweepResult :type Hit%20Result%20Structure%20%28by%20ref%29))
  (bind _asbp_knight (Utilities|Casting|CastToBP_Knight OtherActor))
  (Variables|Default|SetBpKnightRef _asbp_knight)
  (if (Variables|Default|GetIsLastCheckPoint?)
    (CallFunction|LoadNextLevel)
    (else
      (CallFunction|SetRespawnTransform))))

(event Custom|SetRespawnTransform
  (Variables|/Game/Blueprints/BP_Knight.BP_Knight_C|SetSpawnTransform (Variables|Default|GetBpKnightRef) (Transformation|GetWorldTransform (Variables|Default|GetSM_Potato))))

(event Custom|LoadNextLevel
  (bind _returnvalue (UserInterface|CreateWidget "/Game/Blueprints/WB_Win.WB_Win_C"))
  (UserInterface|Viewport|AddtoViewport _returnvalue 0)
  (Utilities|FlowControl|Delay 1.5)
  (Game|OpenLevel(byName) (Variables|Default|GetLevel%20Name)))

(event EventBeginPlay)

(fn ConstructionScript)